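; Procedural room actor that builds a modular room from depth and left/right width settings, entirely in the Construction Script.
; It adds static mesh components to line the side walls and both door walls with WallMesh on WallWidth spacing.
; The exit door frame shifts with depth and the side walls move outward with width.
; Nested loops tile FloorMesh across floors and roofs on a fixed 400-unit grid.
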(fn `GenerateExitDoorWalls`
  (params (Index :type Integer) (IsLeft :type Boolean))
  (locals (LeftWallMultiplyer :type Integer))
  (bind _relativelocation_x (`KismetMathLibrary.BreakVector` (`SceneComponent.RelativeLocation` (`self.ExitDoorsFrame`))))
  (if IsLeft
    (set `local.LeftWallMultiplyer` -1)
    (else
      (set `local.LeftWallMultiplyer` 1)))
  (bind _returnvalue (`AddComponent|NODE_AddStaticMeshComponent-4`))
  (`SceneComponent.K2_SetRelativeLocation` _returnvalue (`KismetMathLibrary.MakeVector` _relativelocation_x (* (+ (* Index (`self.WallWidth`)) 200.0) (`local.LeftWallMultiplyer`))) false false)
  (`StaticMeshComponent.SetStaticMesh` _returnvalue (`self.WallMesh`)))

(fn `GenerateMainDoorWalls`
  (params (Index :type Integer) (IsLeft :type Boolean))
  (locals (LeftWallMultiplyer :type Integer))
  (if IsLeft
    (set `local.LeftWallMultiplyer` -1)
    (else
      (set `local.LeftWallMultiplyer` 1)))
  (bind _returnvalue (`AddComponent|NODE_AddStaticMeshComponent-1`))
  (`SceneComponent.K2_SetRelativeLocation` _returnvalue (`KismetMathLibrary.MakeVector` 0.0 (* (+ (* Index (`self.WallWidth`)) 200.0) (`local.LeftWallMultiplyer`))) false false)
  (`StaticMeshComponent.SetStaticMesh` _returnvalue (`self.WallMesh`)))

(fn `GenerateRoofFloorDepth`
  (params (Parent :type "SceneComponent Object Reference") (Index :type Integer) (IsSide :type Boolean) (IsLeftSide :type "Float (double-precision)"))
  (locals (GeneratedMesh :type "StaticMeshComponent Object Reference"))
  (bind (_relativelocation_x _relativelocation_y _relativelocation_z) (`KismetMathLibrary.BreakVector` (`SceneComponent.RelativeLocation` (`local.GeneratedMesh`))))
  (bind _returnvalue (`AddComponent|NODE_AddStaticMeshComponent-6` :`bManualAttachment` true))
  (bind _output_get (set `local.GeneratedMesh` _returnvalue))
  (`SceneComponent.K2_AttachToComponent` _output_get Parent "None" "SnapToTarget" "SnapToTarget" "SnapToTarget" true)
  (`SceneComponent.K2_SetRelativeLocation` (`local.GeneratedMesh`) (`KismetMathLibrary.MakeVector` (+ _relativelocation_x (* Index 400.0)) 0.0 _relativelocation_z) false false)
  (`StaticMeshComponent.SetStaticMesh` (`local.GeneratedMesh`) (`self.FloorMesh`)))

(fn `GenerateRoofFloorSide`
  (params (Parent :type "SceneComponent Object Reference") (WidthIndex :type Integer) (DepthIndex :type Integer) (IsLeftSide :type "Float (double-precision)"))
  (locals (GeneratedMesh :type "StaticMeshComponent Object Reference"))
  (bind (_relativelocation_x _relativelocation_y _relativelocation_z) (`KismetMathLibrary.BreakVector` (`SceneComponent.RelativeLocation` (`local.GeneratedMesh`))))
  (bind _returnvalue (`AddComponent|NODE_AddStaticMeshComponent-7` :`bManualAttachment` true))
  (bind _output_get (set `local.GeneratedMesh` _returnvalue))
  (`SceneComponent.K2_AttachToComponent` _output_get Parent "None" "SnapToTarget" "SnapToTarget" "SnapToTarget" true)
  (`SceneComponent.K2_SetRelativeLocation` (`local.GeneratedMesh`) (`KismetMathLibrary.MakeVector` (+ _relativelocation_x (* DepthIndex 400.0)) (+ _relativelocation_y (* WidthIndex 400.0 IsLeftSide)) _relativelocation_z) false false)
  (`StaticMeshComponent.SetStaticMesh` (`local.GeneratedMesh`) (`self.FloorMesh`)))

(fn `GenerateSideWalls`
  (params (WallParent :type "SceneComponent Object Reference"))
  (locals (GeneratedWall :type "StaticMeshComponent Object Reference"))
  (for _index (range 1 (+ (`self.DepthRoom`) 1))
    (bind _returnvalue (`AddComponent|NODE_AddStaticMeshComponent-2` :`bManualAttachment` true))
    (bind _output_get (set `local.GeneratedWall` _returnvalue))
    (`SceneComponent.K2_AttachToComponent` _output_get WallParent "None" "SnapToTarget" "SnapToTarget" "SnapToTarget" true)
    (`SceneComponent.K2_SetRelativeLocation` (`local.GeneratedWall`) (`KismetMathLibrary.MakeVector` (.x (`SceneComponent.RelativeLocation` (`local.GeneratedWall`))) (* _index (`self.WallWidth`)) (.z (`SceneComponent.RelativeLocation` (`local.GeneratedWall`)))) false false)
    (`StaticMeshComponent.SetStaticMesh` (`local.GeneratedWall`) (`self.WallMesh`))))

(fn `SetNewLocationExitDoors`
  (bind _relativelocation_x (`KismetMathLibrary.BreakVector` (`SceneComponent.RelativeLocation` (`self.ExitDoorsFrame`))))
  (`SceneComponent.K2_SetRelativeLocation` (`self.ExitDoorsFrame`) (`KismetMathLibrary.MakeVector` (+ _relativelocation_x (* (`self.WallWidth`) (`self.DepthRoom`)))) false false))

(fn `SetNewLocationSideWall`
  (params (SideWall :type "StaticMeshComponent Object Reference") (SideWallWidth :type Integer) (IsLeftWall :type Boolean))
  (locals (RefSideWall :type "StaticMeshComponent Object Reference") (SideWallMultiplyer :type Integer))
  (set `local.RefSideWall` SideWall)
  (if (> SideWallWidth 0)
    (if IsLeftWall
      (set `local.SideWallMultiplyer` -1)
      (else
        (set `local.SideWallMultiplyer` 1)))
    (`SceneComponent.K2_SetRelativeLocation` (`local.RefSideWall`) (`KismetMathLibrary.MakeVector` (.x (`SceneComponent.RelativeLocation` (`local.RefSideWall`))) (* (+ (* (`self.WallWidth`) SideWallWidth) 425.0) (`local.SideWallMultiplyer`))) false false)))

(fn `UserConstructionScript`
  (`|ExecutionSequence`
    (:`then_0`
      ;[0 0 0] Generate Side Walls and set location for exit doors
      (`self.GenerateSideWalls` (`self.MainLeftWall`))
      (`self.GenerateSideWalls` (`self.MainRightWall`))
      (`self.SetNewLocationExitDoors`))
    (:`then_1`
      ;[0 0 0] GenerateWalls
      (for _index (range 1 (+ (`self.RightWallWidth`) 1))
        (`self.GenerateMainDoorWalls` _index)
        (`self.GenerateExitDoorWalls` _index)
        ;[0 0 0] Set New location for side walls
        (`self.SetNewLocationSideWall` (`self.MainRightWall`) (`self.RightWallWidth`))))
    (:`then_2`
      (for _index_2 (range 1 (+ (`self.LeftWallWidth`) 1))
        (`self.GenerateMainDoorWalls` _index_2 true)
        (`self.GenerateExitDoorWalls` _index_2 true)
        (`self.SetNewLocationSideWall` (`self.MainLeftWall`) (`self.LeftWallWidth`) true)))
    (:`then_3`
      ;[0 0 0] Generate depth roofs and floors
      (for _index_3 (range 1 (+ (`self.DepthRoom`) 1))
        (`self.GenerateRoofFloorDepth` (`self.RightRoof`) _index_3 false 1.0)
        (`self.GenerateRoofFloorDepth` (`self.RightFloor`) _index_3 false 1.0)
        (`self.GenerateRoofFloorDepth` (`self.LeftRoof`) _index_3 false 1.0)
        (`self.GenerateRoofFloorDepth` (`self.LeftFloor`) _index_3 false 1.0)))
    (:`then_4`
      ;[0 0 0] Generate right roofs and floors
      (for _index_4 (range (+ (`self.DepthRoom`) 1))
        (for _index_5 (range 1 (+ (`self.RightWallWidth`) 1))
          (`self.GenerateRoofFloorSide` (`self.RightRoof`) _index_5 _index_4 1.0)
          (`self.GenerateRoofFloorSide` (`self.RightFloor`) _index_5 _index_4 1.0))))
    (:`then_5`
      ;[0 0 0] Generate left roofs and floors
      (for _index_6 (range (+ (`self.DepthRoom`) 1))
        (for _index_7 (range 1 (+ (`self.LeftWallWidth`) 1))
          (`self.GenerateRoofFloorSide` (`self.LeftRoof`) _index_7 _index_6 -1.0)
          (`self.GenerateRoofFloorSide` (`self.LeftFloor`) _index_7 _index_6 -1.0))))))